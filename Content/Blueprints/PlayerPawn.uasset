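; PlayerPawn is the player Blueprint, handling HUD creation and the game-over flow.
; On BeginPlay, the locally controlled pawn adds crosshair and health indicator widgets.
; HealthComp's health-change event handles death with a delayed voice cue, game-over widget, disabled movement, pause and mouse cursor.
; Releasing E calls TakeDmage, which subtracts from a separate Health variable and triggers its own immediate game-over screen and pause.
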(event OnHealthChanged(HealthComp)
  (params (HealthComp :type S%20Health%20Component%20Object%20Reference) (Health :type Float%20%28single-precision%29) (HealthDelta :type Float%20%28single-precision%29) (DamageType :type Damage%20Type%20Object%20Reference) (InstigatedBy :type Controller%20Object%20Reference) (DamageCauser :type Actor%20Object%20Reference))
  (if (<= Health 0.0)
    (Utilities|FlowControl|Delay 0.8)
    (Audio|PlaySoundatLocation "/Game/Menus/zapsplat_human_male_voice_says_game_over_004_15729_Cue.zapsplat_human_male_voice_says_game_over_004_15729_Cue" "0, 0, 0" "0, 0, 0" 1.0 1.0 0.0 0 0 0)
    (bind _returnvalue (UserInterface|CreateWidget "/Game/Menus/WBP_GameOver.WBP_GameOver_C"))
    (UserInterface|Viewport|AddtoViewport _returnvalue 0)
    (Pawn|Components|CharacterMovement|DisableMovement (Variables|Character|GetCharacterMovement))
    (Utilities|FlowControl|Delay 1.2)
    (Game|SetGamePaused true)
    (Variables|/Script/Engine.PlayerController|SetbShowMouseCursor (Game|GetPlayerController 0) true)))

(event EventBeginPlay
  (if (Pawn|IsLocallyControlled)
    (Utilities|FlowControl|Sequence
      (:then_0
        (bind _returnvalue (UserInterface|CreateWidget "/Game/UI/WBP_CrossHair.WBP_CrossHair_C"))
        (UserInterface|Viewport|AddtoViewport _returnvalue 0))
      (:then_1
        (bind _returnvalue_2 (UserInterface|CreateWidget "/Game/UI/WBP_HealthIndicator.WBP_HealthIndicator_C"))
        (UserInterface|Viewport|AddtoViewport _returnvalue_2 0)))))

(event Input|KeyboardEvents|E
  (params (Key :type Key%20Structure :default "None"))
  (:Released
    (CallFunction|TakeDmage 1e+02)))

(fn ConstructionScript)

(fn TakeDmage
  (params (DamageTaken :type Float%20%28single-precision%29))
  (bind _output_get (Variables|Default|SetHealth (- (Variables|Default|GetHealth) DamageTaken)))
  (if (<= _output_get 0.0)
    (bind _returnvalue (UserInterface|CreateWidget "/Game/Menus/WBP_GameOver.WBP_GameOver_C"))
    (UserInterface|Viewport|AddtoViewport _returnvalue 0)
    (Game|SetGamePaused true)
    (Variables|/Script/Engine.PlayerController|SetbShowMouseCursor (Game|GetPlayerController 0) true)))